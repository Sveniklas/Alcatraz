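; Trigger Blueprint that shows a one-time WASD controls comment when the player first walks into its Box volume.
; On overlap with the HorrorEngineCharacter, a DoOnce gate waits briefly, adds the WBP_Comment_01WASD_controls widget to the viewport, then removes it after a delay.
; A second box's overlap events are empty, and an older control-scheme widget sequence is left unconnected.
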(event `self.Box.OnComponentBeginOverlap`
  (params (OverlappedComponent :type "PrimitiveComponent Object Reference") (OtherActor :type "Actor Object Reference") (OtherComp :type "PrimitiveComponent Object Reference") (OtherBodyIndex :type Integer) (bFromSweep :type Boolean) (SweepResult :type "HitResult Structure (by ref)"))
  (cast `/Game/HorrorEngine/Blueprints/Core/HorrorEngineCharacter` OtherActor)
  (`/Engine/EditorBlueprintResources/StandardMacros.DoOnce` false
    (:`Completed`
      (`KismetSystemLibrary.Delay` 4.0)
      (bind _returnvalue (`|CreateWidget` "/Game/Blueprints/Comments/Comment_01/WBP_Comment_01-WASD_controls.WBP_Comment_01-WASD_controls_C"))
      (`UserWidget.AddToViewport` _returnvalue 0)
      (`KismetSystemLibrary.Delay` 6.0)
      (`Widget.RemoveFromParent` _returnvalue))))

(event `self.Box1.OnComponentBeginOverlap`
  (params (OverlappedComponent :type "PrimitiveComponent Object Reference") (OtherActor :type "Actor Object Reference") (OtherComp :type "PrimitiveComponent Object Reference") (OtherBodyIndex :type Integer) (bFromSweep :type Boolean) (SweepResult :type "HitResult Structure (by ref)")))

(event `self.Box1.OnComponentEndOverlap`
  (params (OverlappedComponent :type "PrimitiveComponent Object Reference") (OtherActor :type "Actor Object Reference") (OtherComp :type "PrimitiveComponent Object Reference") (OtherBodyIndex :type Integer)))

(fn `UserConstructionScript`)